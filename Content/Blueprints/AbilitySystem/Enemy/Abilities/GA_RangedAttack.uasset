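; Enemy gameplay ability that performs a ranged attack on the avatar's combat target.
; It faces the target, then plays a random tagged attack montage.
; That montage's gameplay event re-reads the target location, spawns a projectile from the tagged socket with optional pitch override, and ends the ability.
; The montage keeps playing after the ability ends; montage completion, interruption or cancellation also ends the ability.
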(event `self.K2_ActivateAbility`
  (bind _returnvalue (message `EnemyInterface.GetCombatTarget` (`self.GetAvatarActorFromActorInfo`)))
  (message `CombatInterface.UpdateFacingTarget` (`self.GetAvatarActorFromActorInfo`) (`Actor.K2_GetActorLocation` _returnvalue))
  (bind _returnvalue_2 (message `CombatInterface.GetAttackMontages` (`self.GetAvatarActorFromActorInfo`)))
  (bind _output_get (set `self.TaggedMontage` (`self.GetRandomTaggedMontageFromArray` _returnvalue_2)))
  (bind (_montage _montagetag) (break `TaggedMontage` _output_get))
  (`AbilityTask_PlayMontageAndWait.CreatePlayMontageAndWaitProxy` "None" _montage 1.0 "None" false
    (:`then`
      (`AbilityTask_WaitGameplayEvent.WaitGameplayEvent` _montagetag null true
        (:`EventReceived`
          (bind _returnvalue_3 (message `EnemyInterface.GetCombatTarget` (`self.GetAvatarActorFromActorInfo`)))
          (`self.SpawnProjectile` (`Actor.K2_GetActorLocation` _returnvalue_3) (`.SocketTag` (break `TaggedMontage` (`self.TaggedMontage`))) (`self.Override Pitch`) 20.0)
          (`self.K2_EndAbility`))))
    (:`OnCompleted`
      (`self.K2_EndAbility` :!label _label))
    (:`OnInterrupted`
      (goto _label))
    (:`OnCancelled`
      (goto _label))))