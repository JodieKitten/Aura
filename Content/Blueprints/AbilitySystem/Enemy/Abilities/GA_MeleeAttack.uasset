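; Enemy melee attack gameplay ability that turns the avatar toward its combat target and plays a randomly chosen tagged attack montage.
; The montage's tag doubles as the gameplay event that triggers the hit, sphere-checking for live players around the matching combat socket.
; Non-friendly players take damage and spawn their blood effect, with one impact sound if anything was hit.
; The ability ends after the hit check or when the montage completes or is interrupted.
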(event `self.K2_ActivateAbility`
  (bind _returnvalue (`self.GetAvatarActorFromActorInfo`))
  (set `self.HasHitTarget` false)
  (bind _returnvalue_2 (message `EnemyInterface.GetCombatTarget` (`self.GetAvatarActorFromActorInfo`)))
  (message `CombatInterface.UpdateFacingTarget` (`self.GetAvatarActorFromActorInfo`) (`Actor.K2_GetActorLocation` _returnvalue_2))
  (bind _returnvalue_3 (message `CombatInterface.GetAttackMontages` (`self.GetAvatarActorFromActorInfo`)))
  (bind _output_get (set `self.TaggedMontage` (`self.GetRandomTaggedMontageFromArray` _returnvalue_3)))
  (bind (_montage _montagetag) (break `TaggedMontage` _output_get))
  (`AbilityTask_PlayMontageAndWait.CreatePlayMontageAndWaitProxy` "None" _montage
    (:`then`
      (`AbilityTask_WaitGameplayEvent.WaitGameplayEvent` _montagetag null
        (:`EventReceived`
          (bind _returnvalue_4 (message `CombatInterface.GetCombatSocketLocation` (`self.GetAvatarActorFromActorInfo`) _montagetag))
          (set `self.CombatSocketLocation` _returnvalue_4)
          (bind _outoverlappingactors (`AuraAbilitySystemLibrary.GetLivePlayersWithinRadius` _returnvalue (`|MakeArray` _returnvalue) 45.0 (`self.CombatSocketLocation`)))
          (for _array_element _outoverlappingactors
            (if (`AuraAbilitySystemLibrary.IsNotFriend` (`self.GetAvatarActorFromActorInfo`) _array_element)
              (`self.CauseDamage` _array_element)
              (set `self.HasHitTarget` true)
              (bind _returnvalue_5 (message `CombatInterface.GetBloodEffect` _array_element))
              (`NiagaraFunctionLibrary.SpawnSystemAtLocation` _returnvalue_5 (`self.CombatSocketLocation`))))
          (if (`self.HasHitTarget`)
            (`GameplayStatics.PlaySoundAtLocation` (`.ImpactSound` (break `TaggedMontage` (`self.TaggedMontage`))) (`self.CombatSocketLocation`) (struct) 1.0 1.0 0.0 null null null null))
          (`self.K2_EndAbility`))))
    (:`OnCompleted`
      (`self.K2_EndAbility` :!label _label))
    (:`OnInterrupted`
      (goto _label))
    (:`OnCancelled`
      (goto _label))))